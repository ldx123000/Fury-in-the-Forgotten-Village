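; BP_BaseItem is a pickup item actor for an inventory system, carrying an ItemInfo struct that the construction script stamps with its own class.
; Its box overlap notifies BP_BaseCharacter when the player enters or leaves, gated by a single Overlap flag on entry.
; Interactive passes ItemInfo to the character and destroys the actor.
; SeeItem shows a nearby-info widget, using DoOnce and a short Delay to hide it and reset.
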(event OnComponentBeginOverlap(Box)
  (params (OverlappedComponent :type Primitive%20Component%20Object%20Reference) (OtherActor :type Actor%20Object%20Reference) (OtherComp :type Primitive%20Component%20Object%20Reference) (OtherBodyIndex :type Integer) (bFromSweep :type Boolean) (SweepResult :type Hit%20Result%20Structure%20%28by%20ref%29))
  ;[1 1 1] Interactive
  (if (not (Variables|Default|GetOverlap))
    (Variables|Default|SetOverlap true)
    (bind _asbp_base_character (Utilities|Casting|CastToBP_BaseCharacter OtherActor))
    (Class|BPIInteractive|Playerin(Message) _asbp_base_character self (Variables|Default|GetItemInfo))))

(event OnComponentEndOverlap(Box)
  (params (OverlappedComponent :type Primitive%20Component%20Object%20Reference) (OtherActor :type Actor%20Object%20Reference) (OtherComp :type Primitive%20Component%20Object%20Reference) (OtherBodyIndex :type Integer))
  ;[1 1 1] Interactive
  (bind _asbp_base_character (Utilities|Casting|CastToBP_BaseCharacter OtherActor))
  (Class|BPIInteractive|PlayerOut(Message) _asbp_base_character self (Variables|Default|GetItemInfo))
  (if (Variables|Default|GetOverlap)
    (Variables|Default|SetOverlap false)))

(event EventInteractive
  (params (Char :type BP%20Base%20Character%20Object%20Reference))
  ;[1 1 1] Pick Up
  (Class|BPIInteractive|PickUp(Message) Char (Variables|Default|GetItemInfo))
  (Actor|DestroyActor))

(event EventSeeItem
  ;[1 1 1] Show Items' Info
  (Utilities|FlowControl|Sequence
    (:then_0
      (Utilities|FlowControl|DoOnce false :!label _label
        (:Completed
          (bind _asui_nearby_item_info (Utilities|Casting|CastToUI_NearbyItemInfo (UserInterface|GetUserWidgetObject (Variables|Default|GetWidget))))
          (Default|SetStyle _asui_nearby_item_info (Variables|Default|GetItemInfo))
          (Rendering|SetVisibility (Variables|Default|GetWidget) true false))))
    (:then_1
      (Utilities|FlowControl|Delay 0.2)
      (Utilities|FlowControl|Sequence
        (:then_0
          (Rendering|SetVisibility (Variables|Default|GetWidget) false false))
        (:then_1
          (goto _label Reset))))))

(fn ConstructionScript
  (Utilities|Struct|SetmembersinBP_ItemInfo (Variables|Default|GetItemInfo) (Utilities|GetClass self)))