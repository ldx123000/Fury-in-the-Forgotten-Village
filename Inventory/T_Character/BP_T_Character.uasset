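; BP_T_Character is an inventory character preview actor that pairs a skeletal mesh with a SceneCaptureComponent2D.
; On BeginPlay it caches player 0's BP_BaseCharacter.
; While that character's IsMouseMoved flag is set, Tick yaws the mesh by MoveUICharacterZ and copies FieldofView to the capture's FOV angle, giving rotation and zoom.
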(event EventBeginPlay
  (bind _asbp_base_character (Utilities|Casting|CastToBP_BaseCharacter (Game|GetPlayerCharacter 0)))
  (Variables|Default|SetCharacterRef _asbp_base_character))

(event Collision|EventActorBeginOverlap
  (params (OtherActor :type Actor%20Object%20Reference)))

(event EventTick
  (params (DeltaSeconds :type Float%20%28single-precision%29))
  (bind _characterref (Variables|Default|GetCharacterRef))
  (if (Variables|/Game/CS3247_2223S2_T7/Inventory/Blueprints/BP_BaseCharacter.BP_BaseCharacter_C|Getis%20Mouse%20Moved _characterref)
    (Transformation|AddRelativeRotation (Variables|Default|GetSkeletalMesh) (Math|Rotator|MakeRotator 0.0 0.0 (Variables|/Game/CS3247_2223S2_T7/Inventory/Blueprints/BP_BaseCharacter.BP_BaseCharacter_C|GetMoveUICharacter_Z _characterref)) false false)
    (Variables|/Script/Engine.SceneCaptureComponent2D|SetFOVAngle (Variables|Default|GetSceneCaptureComponent2D) (Variables|/Game/CS3247_2223S2_T7/Inventory/Blueprints/BP_BaseCharacter.BP_BaseCharacter_C|GetFieldofView _characterref))))

(fn ConstructionScript)