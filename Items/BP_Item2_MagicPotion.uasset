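; Magic potion item Blueprint that restores part of the player hero's MP when its effect runs.
; The Effect event casts player character 0 to BP_HeroBase and adds a quarter of its base MP to current MP, with no clamp here.
; BeginPlay, overlap, tick and construction only call the parent item class.
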(event EventBeginPlay
  (|CallParentFunction))

(event Collision|EventActorBeginOverlap
  (params (OtherActor :type Actor%20Object%20Reference))
  (|CallParentFunction OtherActor))

(event EventTick
  (params (DeltaSeconds :type Float%20%28single-precision%29))
  (|CallParentFunction DeltaSeconds))

(event EventEffect
  (bind _asbp_hero_base (Utilities|Casting|CastToBP_HeroBase (Game|GetPlayerCharacter 0)))
  (Variables|/Game/CS3247_2223S2_T7/Hero/BP_HeroBase.BP_HeroBase_C|SetMP _asbp_hero_base (+ (Variables|/Game/CS3247_2223S2_T7/Hero/BP_HeroBase.BP_HeroBase_C|GetMP _asbp_hero_base) (* (Variables|/Game/CS3247_2223S2_T7/Hero/BP_HeroBase.BP_HeroBase_C|GetMP_base _asbp_hero_base) 0.25))))

(fn ConstructionScript
  (|CallParentFunction))