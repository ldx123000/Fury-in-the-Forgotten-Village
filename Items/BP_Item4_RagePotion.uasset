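; Rage Potion item that triggers the hero's rage when its effect fires.
; The Effect event casts player character 0 to BP_HeroBase and calls Rage on it, doing nothing if the cast fails.
; BeginPlay, overlap, Tick and construction only forward to the parent class, so Effect is the only logic defined here.
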(event EventBeginPlay
  (|CallParentFunction))

(event Collision|EventActorBeginOverlap
  (params (OtherActor :type Actor%20Object%20Reference))
  (|CallParentFunction OtherActor))

(event EventTick
  (params (DeltaSeconds :type Float%20%28single-precision%29))
  (|CallParentFunction DeltaSeconds))

(event EventEffect
  (bind _asbp_hero_base (Utilities|Casting|CastToBP_HeroBase (Game|GetPlayerCharacter 0)))
  (Default|Rage _asbp_hero_base))

(fn ConstructionScript
  (|CallParentFunction))