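; Behavior tree task that moves an AI pawn toward the Target actor from the blackboard.
; Beyond 300 units it issues a move to the target; within that range it issues a move to the pawn itself.
; The task finishes as soon as the move is issued, without waiting for arrival.
; A missing target sets Success to false before finishing, and no branch sets it back to true.
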(event EventReceiveExecuteAI
  (params (OwnerController :type AI%20Controller%20Object%20Reference) (ControlledPawn :type Pawn%20Object%20Reference))
  (bind _asactor (Utilities|Casting|CastToActor (Class|BTFunctionLibrary|GetBlackboardValueasObject (Variables|Default|GetTarget)))
    (:then
      (if (> (Transformation|GetDistanceTo ControlledPawn _asactor) 3e+02)
        (AI|AIMoveTo ControlledPawn "0, 0, 0" _asactor 3e+02 false
          (:then
            _))
        (else
          (AI|AIMoveTo ControlledPawn "0, 0, 0" ControlledPawn 5.0 true
            (:then
              _)))))
    (:CastFailed
      (Variables|Default|SetSuccess false)))
  (AI|BehaviorTree|FinishExecute (Variables|Default|GetSuccess)))