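; Loot component that drops a random potion above its owning actor, using a weighted loot table.
; InjectLootTable supplies a map of item IDs to weights.
; DropLoot totals the weights with CalculateSum, then ChooseLoot rolls within that sum and subtracts each weight until a key is picked.
; The key selects a health, magic, experience or rage potion to spawn, adjusting for collisions.
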(event Custom|DropLoot
  (bind _returnvalue (Components|GetOwner))
  (bind _returnvalue_2 (Transformation|GetActorLocation _returnvalue))
  (bind _returnvalue_3 (+ (.z _returnvalue_2) 1e+02))
  (bind _returnvalue_4 (Math|Vector|MakeVector (.x _returnvalue_2) (.y _returnvalue_2) _returnvalue_3))
  (bind _returnvalue_5 (Math|Transform|MakeTransform _returnvalue_4))
  (bind _sum (CallFunction|CalculateSum))
  (Variables|Default|SetValueSum _sum)
  (bind _loot (CallFunction|ChooseLoot))
  (switch int _loot
    (:1
      (Game|SpawnActorfromClass :Class "/Game/CS3247_2223S2_T7/Items/BP_Item1_HealthPotion.BP_Item1_HealthPotion_C" :SpawnTransform _returnvalue_5 :CollisionHandlingOverride "AdjustIfPossibleButAlwaysSpawn" :Instigator 0))
    (:2
      (Game|SpawnActorfromClass :Class "/Game/CS3247_2223S2_T7/Items/BP_Item2_MagicPotion.BP_Item2_MagicPotion_C" :SpawnTransform _returnvalue_5 :CollisionHandlingOverride "AdjustIfPossibleButAlwaysSpawn" :Instigator 0))
    (:3
      (Game|SpawnActorfromClass :Class "/Game/CS3247_2223S2_T7/Items/BP_Item3_ExpPotion.BP_Item3_ExpPotion_C" :SpawnTransform _returnvalue_5 :CollisionHandlingOverride "AdjustIfPossibleButAlwaysSpawn" :Instigator 0))
    (:4
      (Game|SpawnActorfromClass :Class "/Game/CS3247_2223S2_T7/Items/BP_Item4_RagePotion.BP_Item4_RagePotion_C" :SpawnTransform _returnvalue_5 :CollisionHandlingOverride "AdjustIfPossibleButAlwaysSpawn" :Instigator 0))))

(event Custom|InjectLootTable
  (params (LootTable :type Map%20of%20Integers%20to%20Float%20%28single-precision%29s))
  (Variables|Default|SetLootTable LootTable))

(event EventBeginPlay)

(event EventTick
  (params (DeltaSeconds :type Float%20%28single-precision%29)))

(fn CalculateSum
  (bind _values (Utilities|Map|Values (Variables|Default|GetLootTable)))
  (for _array_element _values
    (bind _output_get (LocalVariables|SetRunningTotal (+ (LocalVariables|GetRunningTotal) _array_element))))
  (return _output_get))

(fn ChooseLoot
  (LocalVariables|SetRandomValue (Math|Random|RandomFloatinRange 0.0 (Variables|Default|GetValueSum)))
  (bind _keys (Utilities|Map|Keys (Variables|Default|GetLootTable)))
  (for _array_element _keys
    (if (<= (LocalVariables|GetRandomValue) (.Value (Utilities|Map|Find (Variables|Default|GetLootTable) _array_element)))
      (return _array_element)
      (else
        (LocalVariables|SetRandomValue (- (LocalVariables|GetRandomValue) (.Value (Utilities|Map|Find (Variables|Default|GetLootTable) _array_element))))))))