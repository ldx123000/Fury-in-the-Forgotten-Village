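; Base hero Blueprint that provides the health bar, pause menu toggle and a timed Rage power-up.
; HeroBeginplay creates the health bar widget, calls CharacterBeginplay and sets two flags.
; The Pause input lazily creates pause and option widgets, then toggles game pause, cursor and input mode.
; Rage enlarges the hero, plays a sound and reverts after a retriggerable delay, while Tick keeps RageATK scaled from ATK.
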(event Custom|Hero%20Beginplay
  (bind _returnvalue (UserInterface|CreateWidget "/Game/CS3247_2223S2_T7/Hero/WarriorHero/Blueprint/BP_HeroHealthBar.BP_HeroHealthBar_C"))
  (bind _output_get (Variables|Default|SetHPRef _returnvalue))
  (UserInterface|Viewport|AddtoViewport _output_get 0)
  (CallFunction|CharacterBeginplay)
  (Variables|Default|Sety_r true)
  (Variables|Default|Sett_r true))

(event Custom|Rage
  (Variables|Default|SetIs_Rage true)
  (Transformation|SetActorRelativeScale3D "1.500000,1.500000,1.500000")
  (Audio|PlaySoundatLocation "/Game/CS3247_2223S2_T7/Enemies/Sevarog/bp_summonsound.bp_summonsound" (Transformation|GetActorLocation) "0, 0, 0" 1.0 1.0 0.0 0 0 0)
  (Utilities|FlowControl|RetriggerableDelay 1e+01)
  (Variables|Default|SetIs_Rage false)
  (Transformation|SetActorRelativeScale3D "1.000000,1.000000,1.000000"))

(event EventBeginPlay
  (|CallParentFunction))

(event Collision|EventActorBeginOverlap
  (params (OtherActor :type Actor%20Object%20Reference))
  (|CallParentFunction OtherActor))

(event EventTick
  (params (DeltaSeconds :type Float%20%28single-precision%29))
  (|CallParentFunction DeltaSeconds)
  (Variables|Default|SetRage_ATK (* (Variables|Default|GetATK) 1.5)))

(event Input|ActionEvents|InputActionPause
  (params (Key :type Key%20Structure :default "None"))
  (bind _returnvalue (Game|GetPlayerController 0))
  (:Pressed
    (Utilities|IsValid (Variables|Default|GetOptionMenuRef)
      (:Is%20Valid
        _)
      (:Is%20Not%20Valid
        (bind _returnvalue_2 (UserInterface|CreateWidget "/Game/CS3247_2223S2_T7/Scene/Menu/bp_option_menu_w.bp_option_menu_w_C"))
        (Variables|Default|SetOptionMenuRef _returnvalue_2)))
    (Utilities|IsValid (Variables|Default|GetPauseMenuRef)
      (:Is%20Valid
        _)
      (:Is%20Not%20Valid
        (bind _returnvalue_3 (UserInterface|CreateWidget "/Game/CS3247_2223S2_T7/Scene/Menu/bp_pause_menu_w.bp_pause_menu_w_C"))
        (Variables|Default|SetPauseMenuRef _returnvalue_3)))
    (if (Game|IsGamePaused)
      (Widget|RemovefromParent (Variables|Default|GetPauseMenuRef))
      (Widget|RemovefromParent (Variables|Default|GetOptionMenuRef))
      (Game|SetGamePaused false)
      (Variables|/Script/Engine.PlayerController|SetbShowMouseCursor _returnvalue false)
      (Input|SetInputModeGameOnly _returnvalue)
      (else
        (UserInterface|Viewport|AddtoViewport (Variables|Default|GetPauseMenuRef) 0)
        (Game|SetGamePaused true)
        (Variables|/Script/Engine.PlayerController|SetbShowMouseCursor _returnvalue true)
        (Input|SetInputModeGameandUI _returnvalue (Variables|Default|GetPauseMenuRef) "LockInFullscreen" false)))))

(fn ConstructionScript)